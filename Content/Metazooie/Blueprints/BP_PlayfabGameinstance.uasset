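; PlayFab game instance Blueprint that hooks dedicated servers into the PlayFab GSDK lifecycle.
; On Init, dedicated servers set the default host port, register GSDK delegates, then signal ReadyForPlayers.
; Shutdown quits the game, and the health check function always reports true.
; Maintenance, server-active and ready-for-players handlers are empty stubs.
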(event Custom|OnGSDKShutdown
  (Game|QuitGame 0 "Quit" false))

(event Custom|OnMaintenanceGSDK
  (params (MaintenanceSchedule :type Maintenance%20Schedule%20Structure%20%28by%20ref%29)))

(event Custom|OnServerActiveGSDK)

(event Custom|OnReadyforPlayersGSDK)

(event EventInit
  (|CallParentFunction)
  (if (Networking|IsDedicatedServer)
    (Class|GSDKUtils|SetDefaultServerHostPort)
    (Class|GSDKUtils|RegisterGSDKShutdownDelegate (delegate Custom|OnGSDKShutdown))
    (Class|GSDKUtils|RegisterGSDKHealthCheckDelegate (EventDispatchers|CreateEvent :!event OnHealthCheckGSDK))
    (Class|GSDKUtils|RegisterGSDKMaintenanceV2Delegate (delegate Custom|OnMaintenanceGSDK))
    (Class|GSDKUtils|RegisterGSDKServerActiveDelegate (delegate Custom|OnServerActiveGSDK))
    (Class|GSDKUtils|RegisterGSDKReadyforPlayers (delegate Custom|OnReadyforPlayersGSDK))
    (Class|GSDKUtils|ReadyforPlayers)))

(fn OnHealthCheckGSDK
  (return true))